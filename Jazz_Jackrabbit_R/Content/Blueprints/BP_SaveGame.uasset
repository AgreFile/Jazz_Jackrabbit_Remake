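; SaveGame object that stores and persists the player's best score for each difficulty.
; SetHighScore forwards to OnSetHighScoreEvent, which compares the new score against the HighScoresForDifficulties map entry for that difficulty.
; A higher score replaces the entry, and the object immediately saves itself to the "HighScores" slot.
; GetHighScores exposes the whole map for reading.
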(event EventSetHighScore
  (params (Difficulty :type E_Difficulties%20Enum :default "NewEnumerator0") (Score :type Float%20%28double-precision%29))
  (CallFunction|OnSetHighScoreEvent Difficulty Score))

(fn OnSetHighScoreEvent
  (params (Difficulty :type E_Difficulties%20Enum%20%28by%20ref%29 :default "NewEnumerator0") (Score :type Float%20%28double-precision%29))
  (LocalVariables|SetDifficultyEnum Difficulty)
  (LocalVariables|SetPointsValue Score)
  (if (< (.Value (Utilities|Map|Find (Variables|Default|GetHighScoresForDifficulties) (LocalVariables|GetDifficultyEnum))) (LocalVariables|GetPointsValue))
    (Utilities|Map|Add (Variables|Default|GetHighScoresForDifficulties) (LocalVariables|GetDifficultyEnum) (LocalVariables|GetPointsValue))
    (SaveGame|SaveGametoSlot self "HighScores")))

(fn GetHighScores
  (return (Variables|Default|GetHighScoresForDifficulties)))