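; BPF_Utils is a utility function library that gives shortcuts to common player and game state queries.
; It checks whether an actor is player character 0 and reads the debug flag and debug trace enum from that character.
; It also sets and reads the game state enum on the current GameState, relying on message calls rather than casts.
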(fn ActorIsPlayer
  (params (Actor :type Actor%20Object%20Reference))
  (return (== Actor (Game|GetPlayerCharacter 0))))

(fn IsDebug
  (bind (_isdebug _debugtraceenum) (Class|BPIUtils|IsDebug(Message) (Game|GetPlayerCharacter 0)))
  (return _isdebug _debugtraceenum))

(fn UpdateGameState
  (params (GameStateE :type E_GameState%20Enum :default "NewEnumerator0"))
  (Class|BPIGameState|UpdateGameStateE(Message) (Game|GetGameState) GameStateE))

(fn GetGameStateE
  (bind _gamestatee (Class|BPIGameState|GetGameStateE(Message) (Game|GetGameState)))
  (return _gamestatee))