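; Base Blueprint for sprite-based interactable signs that react once when shot.
; A Box overlap with a "Bullet"-tagged actor calls Interacted, which sends the sign's enum, itself and Points to player character 0 via SignInteractedMessage.
; It then swaps to InteractedSprite, or only prints a warning if the current sprite is Sign_Sprite.
; Debug prints also flag an unset enum, and WasInteracted blocks repeat hits.
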(event OnComponentBeginOverlap(Box)
  (params (OverlappedComponent :type Primitive%20Component%20Object%20Reference) (OtherActor :type Actor%20Object%20Reference) (OtherComp :type Primitive%20Component%20Object%20Reference) (OtherBodyIndex :type Integer) (bFromSweep :type Boolean) (SweepResult :type Hit%20Result%20Structure%20%28by%20ref%29))
  (if (not (Variables|Default|GetWasInteracted))
    (if (Actor|ActorHasTag OtherActor "Bullet")
      (CallFunction|Interacted))))

(event EventBeginPlay)

(event EventTick
  (params (DeltaSeconds :type Float%20%28single-precision%29)))

(fn ConstructionScript)

(fn Interacted
  (Class|BPIInteractables|SignInteracted(Message) (Game|GetPlayerCharacter 0) (Variables|Default|GetEnum) self (Variables|Default|GetPoints))
  (if (Utilities|Enum|Equal(Enum) (Variables|Default|GetEnum) "NewEnumerator1")
    (Development|PrintString (Utilities|String|Append "WARNING. Interactable with the ingame actor name \"" (Utilities|GetClassDisplayName (Utilities|GetClass self)) "\" has their enum set as NONE") true true "(R=1.000000,G=1.000000,B=0.000000,A=1.000000)" 5.0))
  (if (== (Sprite|GetSprite (Variables|Default|GetRenderComponent)) "/Game/PaperAssets/Interactables/sign_Sprite.sign_Sprite")
    (Development|PrintString (Utilities|String|Append "WARNING. Interactable with the ingame actor name \"" (Utilities|GetClassDisplayName (Utilities|GetClass self)) "\" does not have their InteractedSprite set") true true "(R=1.000000,G=1.000000,B=0.000000,A=1.000000)" 5.0)
    (else
      (Rendering|Components|Sprite|SetSprite (Variables|Default|GetRenderComponent) (Variables|Default|GetInteractedSprite))
      (Development|PrintString "Hello")))
  (Variables|Default|SetWasInteracted true))