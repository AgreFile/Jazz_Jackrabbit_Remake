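; Base 2D Paper flipbook enemy that patrols along the X axis, loading health and damage from the TURTLEGOON row of DT_Enemies.
; A looping timer line-traces for floor ahead and obstacles in front, reversing direction and flipping the sprite.
; Tick drives horizontal movement through physics velocity.
; Box overlap sends the player a hit message, while EnemyHit decrements health and notifies the player before destroying the actor at zero.
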(event OnComponentBeginOverlap(Box)
  (params (OverlappedComponent :type Primitive%20Component%20Object%20Reference) (OtherActor :type Actor%20Object%20Reference) (OtherComp :type Primitive%20Component%20Object%20Reference) (OtherBodyIndex :type Integer) (bFromSweep :type Boolean) (SweepResult :type Hit%20Result%20Structure%20%28by%20ref%29))
  (if (== OtherActor (Game|GetPlayerCharacter 0))
    (Variables|Default|SetplayerInField true)
    (Class|IEnemyInteraction|PlayerHit(Message) (Game|GetPlayerCharacter 0) (Variables|Default|GetDamage) (Transformation|GetActorLocation))))

(event OnComponentEndOverlap(Box)
  (params (OverlappedComponent :type Primitive%20Component%20Object%20Reference) (OtherActor :type Actor%20Object%20Reference) (OtherComp :type Primitive%20Component%20Object%20Reference) (OtherBodyIndex :type Integer))
  (Variables|Default|SetplayerInField false))

(event Custom|CheckFloor
  (bind _returnvalue (Transformation|GetActorLocation))
  (Utilities|FlowControl|Sequence
    (:then_0
      (bind (_outhit _returnvalue_2) (Collision|LineTraceByChannel (+ (Transformation|GetActorLocation) (Math|Vector|MakeVector (* 8e+01 (Variables|Default|Getdirection)) 0.0 0.0)) (+ (+ (Transformation|GetActorLocation) (Math|Vector|MakeVector (* 8e+01 (Variables|Default|Getdirection)) 0.0 0.0)) "0.000000,0.000000,-90.000000") "TraceTypeQuery1" false 0 (Variables|Default|GetDebugTraceEnum) true "(R=1.000000,G=0.000000,B=0.000000,A=1.000000)" "(R=0.000000,G=1.000000,B=0.000000,A=1.000000)" 0.05))
      (if (or (Utilities|Operators|NotEqual(!=) (.impactnormal _outhit) "0.000000,0.000000,1.000000" 0.001) (!= _returnvalue_2 true))
        (Variables|Default|Setdirection (* (Variables|Default|Getdirection) -1.0))
        (if (> (Variables|Default|Getdirection) 0.0) :!label _label
          (Transformation|SetRelativeRotation (Variables|Default|GetPaperFlipbook) "0.000000,180.000000,0.000000" false false)
          (else
            (Transformation|SetRelativeRotation (Variables|Default|GetPaperFlipbook) "0, 0, 0" false false)))))
    (:then_1
      (bind _returnvalue_3 (Collision|LineTraceByChannel _returnvalue (+ _returnvalue (Math|Vector|MakeVector (* 1.1e+02 (Variables|Default|Getdirection)) 0.0 0.0)) "TraceTypeQuery1" false 0 "ForOneFrame" true "(R=1.000000,G=0.000000,B=0.000000,A=1.000000)" "(R=0.000000,G=1.000000,B=0.000000,A=1.000000)" 0.05))
      (if _returnvalue_3
        (Variables|Default|Setdirection (* (Variables|Default|Getdirection) -1.0))
        (goto _label)))))

(event EventBeginPlay
  (bind _returnvalue (Utilities|GetDataTableRow "/Game/Data/DT_Enemies.DT_Enemies" "TURTLEGOON")
    (:then
      (CallFunction|SetEnemyData _returnvalue)
      (Utilities|Time|SetTimerbyEvent (delegate Custom|CheckFloor) 0.05 true)
      (bind (_isdebug _debugtraceenum) (CallFunction|IsDebug))
      (Variables|Default|SetIsDebug _isdebug)
      (Variables|Default|SetDebugTraceEnum _debugtraceenum)
      (Transformation|SetRelativeRotation (Variables|Default|GetPaperFlipbook) "0.000000,180.000000,0.000000" false false))))

(event Collision|EventActorBeginOverlap
  (params (OtherActor :type Actor%20Object%20Reference)))

(event EventTick
  (params (DeltaSeconds :type Float%20%28single-precision%29))
  (bind _rendercomponent (Variables|Default|GetRenderComponent))
  (bind _returnvalue (Transformation|GetComponentVelocity _rendercomponent))
  (Class|PrimitiveComponent|SetAllPhysicsLinearVelocity _rendercomponent (Math|Vector|MakeVector (* (Variables|Default|Getspeed) (Variables|Default|Getdirection)) (.y _returnvalue) (.z _returnvalue)) false))

(event EventEnemyHit
  (bind _result (Math|Float|DecrementFloat (Variables|Default|GetHealth))
    (:%20%20
      (if (<= _result 0.0)
        (Class|IEnemyInteraction|EnemyKilled(Message) (Game|GetPlayerCharacter 0))
        (Actor|DestroyActor)))))

(fn ConstructionScript)

(fn SetEnemyData
  (params (EnemyStruct :type S%20Enemy%20Structure))
  (Variables|Default|SetHealth (.health EnemyStruct))
  (Variables|Default|SetDamage (.damage EnemyStruct)))