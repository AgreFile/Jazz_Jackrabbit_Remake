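; Flying 2D enemy that drifts in a wavy pattern, hurts the player on contact and dies when its health runs out.
; BeginPlay loads health and damage from the TURTLEGOON row of DT_Enemies, then starts a fast looping timer for Fly.
; Fly offsets the render component with sine waves on X and Z and flips the flipbook to match horizontal direction.
; Box overlap sends damage to the player, while EnemyHit decrements health and reports the kill before destroying itself.
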(event OnComponentBeginOverlap(Box)
  (params (OverlappedComponent :type Primitive%20Component%20Object%20Reference) (OtherActor :type Actor%20Object%20Reference) (OtherComp :type Primitive%20Component%20Object%20Reference) (OtherBodyIndex :type Integer) (bFromSweep :type Boolean) (SweepResult :type Hit%20Result%20Structure%20%28by%20ref%29))
  (if (== OtherActor (Game|GetPlayerCharacter 0))
    (Variables|Default|SetplayerInField true)
    (Class|IEnemyInteraction|PlayerHit(Message) (Game|GetPlayerCharacter 0) (Variables|Default|GetDamage) (Transformation|GetActorLocation))))

(event OnComponentEndOverlap(Box)
  (params (OverlappedComponent :type Primitive%20Component%20Object%20Reference) (OtherActor :type Actor%20Object%20Reference) (OtherComp :type Primitive%20Component%20Object%20Reference) (OtherBodyIndex :type Integer))
  (Variables|Default|SetplayerInField false))

(event Custom|Fly
  (bind _returnvalue (Utilities|Time|GetGameTimeinSeconds))
  (bind _paperflipbook (Variables|Default|GetPaperFlipbook))
  (bind _returnvalue_2 (* _returnvalue 0.5))
  (bind _returnvalue_3 (Math|Trig|Sin(Radians) _returnvalue_2))
  (Transformation|AddLocalOffset (Variables|Default|GetRenderComponent) (Math|Vector|MakeVector (* _returnvalue_3 0.5) 0.0 (* (Math|Trig|Sin(Radians) (* _returnvalue 1.785)) 0.264)) false false)
  (if (> _returnvalue_3 0.0)
    (Transformation|SetRelativeRotation _paperflipbook "0.000000,180.000000,0.000000" false false)
    (else
      (Transformation|SetRelativeRotation _paperflipbook "0, 0, 0" false false))))

(event EventBeginPlay
  (bind _returnvalue (Utilities|GetDataTableRow "/Game/Data/DT_Enemies.DT_Enemies" "TURTLEGOON")
    (:then
      (CallFunction|SetEnemyData _returnvalue)
      (Utilities|Time|SetTimerbyEvent (delegate Custom|Fly) 0.01 true)
      (bind (_isdebug _debugtraceenum) (CallFunction|IsDebug))
      (Variables|Default|SetIsDebug _isdebug)
      (Variables|Default|SetDebugTraceEnum _debugtraceenum)
      (Transformation|SetRelativeRotation (Variables|Default|GetPaperFlipbook) "0.000000,180.000000,0.000000" false false))))

(event Collision|EventActorBeginOverlap
  (params (OtherActor :type Actor%20Object%20Reference)))

(event EventEnemyHit
  (bind _result (Math|Float|DecrementFloat (Variables|Default|GetHealth))
    (:%20%20
      (if (<= _result 0.0)
        (Class|IEnemyInteraction|EnemyKilled(Message) (Game|GetPlayerCharacter 0))
        (Actor|DestroyActor)))))

(fn ConstructionScript)

(fn SetEnemyData
  (params (EnemyStruct :type S%20Enemy%20Structure))
  (Variables|Default|SetHealth (.health EnemyStruct))
  (Variables|Default|SetDamage (.damage EnemyStruct)))