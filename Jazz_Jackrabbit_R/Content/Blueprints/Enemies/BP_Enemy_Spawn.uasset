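; Enemy spawner sprite actor that places a turtle goon in the level, gated by difficulty.
; The construction script applies the sprite and scale from the hardcoded TURTLEGOON row in DT_Enemies, so the placed spawner previews its enemy.
; On BeginPlay, it spawns that row's actor class at its own location and rotation with the row's scale, if the current difficulty meets or exceeds its Difficulty setting.
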(event EventBeginPlay
  (bind _returnvalue (Transformation|GetActorTransform))
  (bind (_location _rotation) (Math|Transform|BreakTransform _returnvalue))
  (if (>= (Math|Byte|MakeLiteralByte (CallFunction|GetDifficulty)) (Math|Byte|MakeLiteralByte (Variables|Default|GetDifficulty)))
    (bind _returnvalue_2 (Utilities|GetDataTableRow "/Game/Data/DT_Enemies.DT_Enemies" "TURTLEGOON")
      (:then
        (Game|SpawnActorfromClass (.actorclass _returnvalue_2) (Math|Transform|MakeTransform _location _rotation (.scale _returnvalue_2)) "Undefined" "MultiplyWithRoot" 0 0)))))

(event Collision|EventActorBeginOverlap
  (params (OtherActor :type Actor%20Object%20Reference)))

(event EventTick
  (params (DeltaSeconds :type Float%20%28single-precision%29)))

(fn ConstructionScript
  (bind _returnvalue (Utilities|GetDataTableRow "/Game/Data/DT_Enemies.DT_Enemies" "TURTLEGOON")
    (:then
      (Rendering|Components|Sprite|SetSprite (Variables|Default|GetRenderComponent) (.sprite _returnvalue))
      (Transformation|SetActorScale3D (.scale _returnvalue)))))