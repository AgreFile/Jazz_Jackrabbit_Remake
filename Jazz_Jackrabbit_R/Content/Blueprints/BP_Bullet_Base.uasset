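; Base pooled bullet actor fired by the player that notifies enemy-tagged actors when it overlaps them.
; Shoot teleports the physics box to the spawn transform and launches it along the facing direction, adding the player's horizontal speed and a bullet angle.
; A looping timer, paused while idle, enforces lifetime.
; Expiry or any valid overlap triggers Deactivate, which parks the bullet far away and returns its index and weapon type to the player character.
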(event Custom|LifetimeTimerEvent
  (if (> (- (Utilities|Time|GetGameTimeinSeconds) (Variables|Default|GetStartTime)) (Variables|Default|GetLifetime))
    (CallFunction|Deactivate)))

(event EventBeginPlay
  (bind _returnvalue (Utilities|Time|SetTimerbyEvent (delegate Custom|LifetimeTimerEvent) 0.1 true))
  (bind _output_get (Variables|Default|SettimerHandle _returnvalue))
  (Utilities|Time|PauseTimerbyHandle _output_get))

(event Collision|EventActorBeginOverlap
  (params (OtherActor :type Actor%20Object%20Reference))
  (if (Utilities|IsValid OtherActor)
    (if (Actor|ActorHasTag OtherActor "enemy")
      (Class|IEnemyInteraction|EnemyHit(Message) OtherActor))
    (CallFunction|Deactivate)))

(event EventTick
  (params (DeltaSeconds :type Float%20%28single-precision%29)))

(event EventShoot
  (params (bulletVelocity :type Vector :default "0, 0, 0") (playerVel :type Vector :default "0, 0, 0") (spawnPos :type Transform) (playerOrientationMultiplier :type Float%20%28double-precision%29) (ArrayIndex :type Integer) (Weapon :type E_Weapons%20Enum :default "NewEnumerator0") (BulletAngle :type Float%20%28double-precision%29))
  (Utilities|Time|UnpauseTimerbyHandle (Variables|Default|GettimerHandle))
  (Variables|Default|SetPlayer%20Orientation%20Multiplier playerOrientationMultiplier)
  (Variables|Default|SetStartTime (Utilities|Time|GetGameTimeinSeconds))
  (Variables|Default|SetArrayIndex ArrayIndex)
  (Variables|Default|SetWeaponEnum Weapon)
  (Transformation|SetWorldTransform (Variables|Default|GetBox) spawnPos false false)
  (Physics|SetPhysicsLinearVelocity (Variables|Default|GetBox) (Math|Vector|RotateVector (Math|Vector|MakeVector (* (+ 2.5e+03 (Math|Float|Absolute(Float) (.X (Math|Vector|BreakVector playerVel)))) (Variables|Default|GetPlayer%20Orientation%20Multiplier)) 0.0 0.0) (Math|Rotator|MakeRotator 0.0 BulletAngle 0.0)) false "None"))

(fn ConstructionScript)

(fn Deactivate
  (bind _box (Variables|Default|GetBox))
  (Utilities|Time|PauseTimerbyHandle (Variables|Default|GettimerHandle))
  (Physics|SetPhysicsLinearVelocity _box (Math|Vector|MakeVector 0.0 0.0 0.0) false "None")
  (Transformation|SetWorldLocation _box "100000.000000,100000.000000,100000.000000" false false)
  (Class|BPIBullets|DeactivateBullet(Message) (Game|GetPlayerCharacter 0) (Variables|Default|GetArrayIndex) (Variables|Default|GetWeaponEnum)))