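; BP_MainMenuCharacter is the player Blueprint for the main menu, hosting the menu UI.
; On BeginPlay it creates the main menu, options and level selection widgets, adds all three to the viewport and shows the mouse cursor.
; Its OpenSettings and OpenLevels events forward to the stored options and level selection widgets by calling their open-message functions.
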(event EventBeginPlay
  (bind _returnvalue (UserInterface|CreateWidget "/Game/Blueprints/UI/MainMenu/WBP_MainMenu.WBP_MainMenu_C"))
  (bind _output_get (Variables|Default|SetMainMenuRef _returnvalue))
  (UserInterface|Viewport|AddtoViewport _output_get 0)
  (bind _returnvalue_2 (UserInterface|CreateWidget "/Game/Blueprints/UI/MainMenu/WBP_Options.WBP_Options_C"))
  (bind _output_get_2 (Variables|Default|SetOptionsRef _returnvalue_2))
  (UserInterface|Viewport|AddtoViewport _output_get_2 0)
  (Variables|/Script/Engine.PlayerController|SetbShowMouseCursor (Game|GetPlayerController 0) true)
  (bind _returnvalue_3 (UserInterface|CreateWidget "/Game/Blueprints/UI/MainMenu/WBP_LevelSelection.WBP_LevelSelection_C"))
  (bind _output_get_3 (Variables|Default|SetLevelsRef _returnvalue_3))
  (UserInterface|Viewport|AddtoViewport _output_get_3 0))

(event Collision|EventActorBeginOverlap
  (params (OtherActor :type Actor%20Object%20Reference)))

(event EventTick
  (params (DeltaSeconds :type Float%20%28single-precision%29)))

(event EventOpenSettings
  (Class|IUiInterface|OpenSettings(Message) (Variables|Default|GetOptionsRef)))

(event EventOpenLevels
  (Class|IUiInterface|OpenLevels(Message) (Variables|Default|GetLevelsRef)))

(fn ConstructionScript)