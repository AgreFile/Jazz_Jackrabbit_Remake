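; Base Blueprint for collectibles, meant to be subclassed with specific pickup behavior.
; Overlap of its Box with player character 0 calls Collect, which only prints a missing-override message by default; CollectEnd destroys the actor.
; A waving event bobs RenderComponent on a sine of game time plus a per-instance random phase, but nothing here triggers it: the timer is disconnected and the ShouldWave branch is empty.
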(event OnComponentBeginOverlap(Box)
  (params (OverlappedComponent :type Primitive%20Component%20Object%20Reference) (OtherActor :type Actor%20Object%20Reference) (OtherComp :type Primitive%20Component%20Object%20Reference) (OtherBodyIndex :type Integer) (bFromSweep :type Boolean) (SweepResult :type Hit%20Result%20Structure%20%28by%20ref%29))
  (if (== OtherActor (Game|GetPlayerCharacter 0))
    (CallFunction|Collect)))

(event OnComponentBeginOverlap(RenderComponent)
  (params (OverlappedComponent :type Primitive%20Component%20Object%20Reference) (OtherActor :type Actor%20Object%20Reference) (OtherComp :type Primitive%20Component%20Object%20Reference) (OtherBodyIndex :type Integer) (bFromSweep :type Boolean) (SweepResult :type Hit%20Result%20Structure%20%28by%20ref%29)))

(event Custom|waving
  (Transformation|AddLocalOffset (Variables|Default|GetRenderComponent) (Math|Vector|MakeVector 0.0 0.0 (* (Math|Trig|Sin(Radians) (* (+ (Utilities|Time|GetGameTimeinSeconds) (Variables|Default|GetRandomness)) 3.0)) 1.0)) false false))

(event EventBeginPlay
  (Variables|Default|SetRandomness (Math|Random|RandomFloatinRange -1e+02 1e+02))
  (if (Variables|Default|GetshouldWave)
    _))

(event Collision|EventActorBeginOverlap
  (params (OtherActor :type Actor%20Object%20Reference)))

(event EventTick
  (params (DeltaSeconds :type Float%20%28single-precision%29)))

(fn ConstructionScript)

(fn CollectEnd
  (Actor|DestroyActor))

(fn Collect
  (Development|PrintString (Utilities|String|Append "Collectible " (Utilities|GetObjectName self) " doesn't have its Collect function overridden")))