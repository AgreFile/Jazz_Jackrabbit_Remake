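; BP_C_SecretSparkle is a collectible, by name the secret sparkle variant, built on a parent class that handles the shared behavior.
; Its Collect function sends the player character a collected message with this collectible's type enum, then calls CollectEnd.
; BeginPlay, overlap, Tick and the construction script only forward to the parent.
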(event EventBeginPlay
  (|CallParentFunction))

(event Collision|EventActorBeginOverlap
  (params (OtherActor :type Actor%20Object%20Reference))
  (|CallParentFunction OtherActor))

(event EventTick
  (params (DeltaSeconds :type Float%20%28single-precision%29))
  (|CallParentFunction DeltaSeconds))

(fn ConstructionScript
  (|CallParentFunction))

(fn Collect
  (Class|ICollectibles|CollectibleCollected(Message) (Game|GetPlayerCharacter 0) "NewEnumerator2")
  (CallFunction|CollectEnd))