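; Ammo pickup collectible that grants the player an amount of ammo for a given weapon type.
; On BeginPlay it runs the parent setup and sets its points value.
; Collect sends the weapon type and amount to player character 0 through AmmoCollectedMessage, then calls CollectEnd to finish the pickup.
; The weapon switches in BeginPlay and the construction script have no actions attached.
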(event EventBeginPlay
  (|CallParentFunction)
  (Variables|Default|SetPointsValue 1e+02)
  (switch Utilities|FlowControl|Switch|SwitchonE_Weapons (Variables|Default|GetWeapon)))

(event Collision|EventActorBeginOverlap
  (params (OtherActor :type Actor%20Object%20Reference))
  (|CallParentFunction OtherActor) ; This node is disabled and will not be called.\nDrag off pins to build functionality.
)

(event EventTick
  (params (DeltaSeconds :type Float%20%28single-precision%29))
  (|CallParentFunction DeltaSeconds) ; This node is disabled and will not be called.\nDrag off pins to build functionality.
)

(fn ConstructionScript
  (|CallParentFunction)
  (switch Utilities|FlowControl|Switch|SwitchonE_Weapons "NewEnumerator0"))

(fn Collect
  (Class|ICollectibles|AmmoCollected(Message) (Game|GetPlayerCharacter 0) (Variables|Default|GetWeapon) (Variables|Default|GetAmount))
  (CallFunction|CollectEnd))