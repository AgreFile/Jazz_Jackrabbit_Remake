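; BP_C_Basic is a data-driven collectible with a sprite, configured by its Collectible enum.
; The construction script scans DT_Collectibles for rows matching that enum, then copies their points value and sprite onto the actor.
; Collect sends the collectible type to the player character through CollectibleCollectedMessage, then calls CollectEnd.
; The event graph holds only disabled default events.
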(event EventBeginPlay
  (|CallParentFunction) ; This node is disabled and will not be called.\nDrag off pins to build functionality.
)

(event Collision|EventActorBeginOverlap
  (params (OtherActor :type Actor%20Object%20Reference))
  (|CallParentFunction OtherActor) ; This node is disabled and will not be called.\nDrag off pins to build functionality.
)

(event EventTick
  (params (DeltaSeconds :type Float%20%28single-precision%29))
  (|CallParentFunction DeltaSeconds) ; This node is disabled and will not be called.\nDrag off pins to build functionality.
)

(fn ConstructionScript
  (|CallParentFunction)
  (bind _outrownames (DataTable|GetDataTableRowNames "/Game/Data/DT_Collectibles.DT_Collectibles"))
  (bind _array_element (Utilities|Array|ForEachLoopwithBreak _outrownames)
    (:LoopBody
      (bind _returnvalue (Utilities|GetDataTableRow "/Game/Data/DT_Collectibles.DT_Collectibles" _array_element)
        (:then
          (if (Utilities|Enum|Equal(Enum) (Variables|Default|GetCollectible) (.enum _returnvalue))
            (Variables|Default|SetPointsValue (.pointstoadd _returnvalue))
            (Rendering|Components|Sprite|SetSprite (Variables|Default|GetRenderComponent) (.sprite _returnvalue))))))))

(fn Collect
  (Class|ICollectibles|CollectibleCollected(Message) (Game|GetPlayerCharacter 0) (Variables|Default|GetCollectible))
  (CallFunction|CollectEnd))